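; Actor that visualizes one tracked eye, left or right per its Eye setting, in an eye position example.
; Each tick it shows the eye sphere only while the user is present, and updates the stored position only when that eye's data is valid.
; It interpolates toward the scaled position, rotates to face the 3D gaze point actor and draws a debug line to it.
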(event `self.ReceiveTick`
  (params (DeltaSeconds :type "Float (single-precision)"))
  (bind (_lefteye _righteye _bislefteyevalid _bisrighteyevalid) (`EyeXBlueprintLibrary.GetEyePosition`))
  (bind _returnvalue (`self.K2_GetActorLocation`))
  (bind _returnvalue_2 (`self.K2_GetActorLocation` (`self.3DGazePoint`)))
  (bind _returnvalue_3 (`|EnumEquality` (`EyeXBlueprintLibrary.GetUserPresence`) "Present"))
  ;[1 1 1] If the user is not present, hide the eye and don't do anything else
  (`SceneComponent.SetVisibility` (`self.EyeSphere`) _returnvalue_3 false)
  (if _returnvalue_3
    (`|ExecutionSequence`
      (:`then_0`
        ;[1 1 1] Update new eye position if it's valid
        (switch `/Game/Blueprints/EyePositionExample/EEye` (`self.Eye`)
          (:`NewEnumerator0`
            (if _bislefteyevalid
              (set `self.EyePosition` _lefteye)))
          (:`NewEnumerator1`
            (if _bisrighteyevalid
              (set `self.EyePosition` _righteye)))))
      (:`then_1`
        ;[1 1 1] Move towards new eye position
        (`self.K2_SetActorLocation` (`KismetMathLibrary.VInterpTo` (`self.K2_GetActorLocation`) (* (`self.EyePosition`) 10.0) (`GameplayStatics.GetWorldDeltaSeconds`) (`self.InterpSpeed`))))
      (:`then_2`
        ;[1 1 1] Rotate eyeballs and draw line from eyeball to the 3D gaze position
        (`self.SetActorRotation` (`KismetMathLibrary.FindLookAtRotation` _returnvalue _returnvalue_2))
        (`KismetSystemLibrary.DrawDebugLine` _returnvalue _returnvalue_2 (struct :`R` 0.116576 :`G` 0.22331 :`B` 1.0 :`A` 1.0))))))

(fn `UserConstructionScript`)