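; HUD for the eye position example, showing an "Eye Positions" title with help text and outlining the viewport as a 3D debug rectangle.
; Each DrawHUD converts the viewport corners from pixels to millimeters using the display size and screen bounds.
; The corners are centered on the origin in the X=0 plane, matching the coordinate system of the 3D gaze point and eye position.
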(event `self.ReceiveDrawHUD`
  (params (SizeX :type Integer) (SizeY :type Integer))
  (bind (_displaysize _bhasvalue) (`EyeXBlueprintLibrary.GetDisplaySize`))
  (bind (_x _y _width _height _bhasvalue_2) (`EyeXBlueprintLibrary.GetScreenBounds`))
  (bind _viewportcorners (`self.ViewportCorners`))
  (bind (_x_2 _y_2) (`KismetMathLibrary.BreakVector2D` _displaysize))
  (bind _returnvalue (/ (`KismetMathLibrary.Conv_IntToDouble` SizeX) 2.0))
  (bind _returnvalue_2 (/ (`KismetMathLibrary.Conv_IntToDouble` SizeY) 2.0))
  (bind _returnvalue_3 (* _returnvalue -1.0))
  (bind _returnvalue_4 (* _returnvalue_2 -1.0))
  ;[1 1 1] Print help text
  (bind (_screen_x _screen_y _outwidth _outheight) (`/Game/Blueprints/BPMacroLibrary.DrawCenteredTextOnHUD` (/ SizeX 2) (/ SizeY 3) "Eye Positions" (struct :`R` 1.0 :`G` 1.0 :`B` 1.0 :`A` 1.0) "/Game/Fonts/Calibri.Calibri")
    (:`  `
      (`self.DrawText` (`self.HelpText`) (struct :`R` 1.0 :`G` 1.0 :`B` 1.0 :`A` 1.0) _screen_x (+ _screen_y _outheight) "/Game/Fonts/Calibri_small.Calibri_small")
      ;[1 1 1] Convert to 3D-coordinates in the same coordinate system used by the 3D Gaze point and the eye position
      (for _array_element (`|MakeArray` (`KismetMathLibrary.MakeVector2D` _returnvalue _returnvalue_2) (`KismetMathLibrary.MakeVector2D` _returnvalue _returnvalue_4) (`KismetMathLibrary.MakeVector2D` _returnvalue_3 _returnvalue_4) (`KismetMathLibrary.MakeVector2D` _returnvalue_3 _returnvalue_2))
        (if (and _bhasvalue _bhasvalue_2)
          (bind (_x_3 _y_3) (`KismetMathLibrary.BreakVector2D` _array_element))
          (`KismetArrayLibrary.Array_Add` (`self.ViewportCorners`) (`KismetMathLibrary.MakeVector` 0.0 (* _x_3 (/ _x_2 (`KismetMathLibrary.Conv_IntToDouble` _width))) (* (* _y_3 (/ _y_2 (`KismetMathLibrary.Conv_IntToDouble` _height))) -1.0)))))
      ;[1 1 1] Draw a rectangle using the corners of the viewport
      (if (== (`KismetArrayLibrary.Array_Length` (`self.ViewportCorners`)) 4)
        (for _index (range 4)
          (`KismetSystemLibrary.DrawDebugLine` (`KismetArrayLibrary.Array_Get` _viewportcorners _index) (`KismetArrayLibrary.Array_Get` _viewportcorners (mod (+ _index 1) 4)) (struct :`R` 0.116576 :`G` 0.22331 :`B` 1.0 :`A` 1.0)))
        (`KismetArrayLibrary.Array_Clear` (`self.ViewportCorners`))))))

(fn `UserConstructionScript`)