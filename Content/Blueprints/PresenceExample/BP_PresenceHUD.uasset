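; Example HUD that shows on screen whether the user is detected as present.
; Each DrawHUD reads the user presence state and draws a centered message for Present, Not Present or Unknown.
; Not Present and Unknown share one branch that dims the screen with a translucent black rectangle and uses gray text.
; A feature description is then drawn just below the message in the matching color and a smaller font.
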(event `self.ReceiveDrawHUD`
  (params (SizeX :type Integer) (SizeY :type Integer))
  (bind _black (`self.Black`))
  (bind _darkgray (`self.DarkGray`))
  (set `self.HUDSizeX` SizeX)
  (set `self.HUDSizeY` SizeY)
  (switch `EEyeXUserPresence` (`EyeXBlueprintLibrary.GetUserPresence`)
    (:`Present`
      ;[1 1 1] User is present
      (set `self.DescriptionTextColor` _black)
      (bind (_screen_x _screen_y _outwidth _outheight) (`/Game/Blueprints/BPMacroLibrary.DrawCenteredTextOnHUD` (`self.HUDSizeX`) (`self.HUDSizeY`) "Hi, I can see you are here!" _black "/Game/Fonts/Calibri.Calibri")
        (:`  `
          (set `self.DescriptionScreenX` _screen_x)
          (set `self.DescriptionScreenY` (+ _screen_y _outheight 0.0)))))
    (:`NotPresent`
      ;[1 1 1] User precense is Unknown or Not Present
      (set `self.Message` "Ok, where did you go? I'll wait...")
      (`self.DrawRect` (struct :`A` 0.8) 0.0 0.0 (`KismetMathLibrary.Conv_IntToDouble` (`self.HUDSizeX`)) (`KismetMathLibrary.Conv_IntToDouble` (`self.HUDSizeY`)) :!label _label)
      (set `self.DescriptionTextColor` _darkgray)
      (bind (_screen_x_2 _screen_y_2 _outwidth_2 _outheight_2) (`/Game/Blueprints/BPMacroLibrary.DrawCenteredTextOnHUD` (`self.HUDSizeX`) (`self.HUDSizeY`) (`self.Message`) _darkgray "/Game/Fonts/Calibri.Calibri")
        (:`  `
          (set `self.DescriptionScreenX` _screen_x_2)
          (set `self.DescriptionScreenY` (+ _screen_y_2 _outheight_2 0.0)))))
    (:`Unknown`
      (set `self.Message` "Don't know if you are here or not...")
      (goto _label)))
  (`self.DrawText` (`self.FeatureDescription`) (`self.DescriptionTextColor`) (`self.DescriptionScreenX`) (`self.DescriptionScreenY`) "/Game/Fonts/Calibri_small.Calibri_small"))

(fn `UserConstructionScript`)