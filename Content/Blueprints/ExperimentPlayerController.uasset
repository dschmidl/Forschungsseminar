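; Player controller for a gaze-controlled car interface experiment, with cruise control, navigation, infotainment and climate menus.
; BeginPlay creates the MainView widget, and Tick tests the filtered eye-tracker gaze point against hard-coded screen rectangles, one per menu.
; A gazed menu turns red and gives keyboard focus to the button at its key counter; otherwise its indicator turns dark.
; Separate events show incoming call, message and navigation notifications after a short delay.
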(event `self.ReceiveTick`
  (params (DeltaSeconds :type "Float (single-precision)"))
  (bind (_x _y) (`KismetMathLibrary.BreakVector2D` (`EyeXBlueprintLibrary.GetGazePoint` "LightlyFiltered")))
  (bind _tempomat_menu_45 (`/Game/UMG/MainView.Tempomat_Menu_45` (`self.MainViewWidgetReference`)))
  (bind _navi_menu_65 (`/Game/UMG/MainView.Navi_Menu_65` (`self.MainViewWidgetReference`)))
  (bind _infotainment_menu_72 (`/Game/UMG/MainView.Infotainment_Menu_72` (`self.MainViewWidgetReference`)))
  (bind _klima_menu (`/Game/UMG/MainView.Klima_Menu` (`self.MainViewWidgetReference`)))
  (bind _returnvalue (`KismetMathLibrary.FTrunc` _y))
  (bind _returnvalue_2 (`KismetMathLibrary.FTrunc` _x))
  (bind _button_302 (`/Game/UMG/Tempomat_menu.Button_302` _tempomat_menu_45))
  (bind _tempomatbuttondown10 (`/Game/UMG/Tempomat_menu.TempomatButtonDown10` _tempomat_menu_45))
  (bind _urbutton (`/Game/UMG/Navi_Menu.URButton` _navi_menu_65))
  (bind _button_302_2 (`/Game/UMG/Navi_Menu.Button_302` _navi_menu_65))
  (bind _klimaminusbutton (`/Game/UMG/Klima_Menu.KlimaMinusButton` _klima_menu))
  (bind _mainradiobutton (`/Game/UMG/Infotainment_Menu.MainRadioButton` (`/Game/UMG/MainView.Infotainment_Menu_72` (`self.MainViewWidgetReference`))))
  (bind _mainradiobutton_2 (`/Game/UMG/Infotainment_Menu.MainRadioButton` _infotainment_menu_72))
  (bind _image_72 (`/Game/UMG/Klima_Menu.Image_72` _klima_menu))
  (bind _item (`KismetArrayLibrary.Array_Get` (`|MakeArray` _tempomatbuttondown10 (`/Game/UMG/Tempomat_menu.TempomatButtonDown1` _tempomat_menu_45) (`/Game/UMG/Tempomat_menu.TempomatButtonUp1` _tempomat_menu_45) (`/Game/UMG/Tempomat_menu.TempomatButtonUp10` _tempomat_menu_45)) (`/Game/UMG/Tempomat_menu.KeyCounter` _tempomat_menu_45)))
  (bind _item_2 (`KismetArrayLibrary.Array_Get` (`|MakeArray` _mainradiobutton_2 (`/Game/UMG/Infotainment_Menu.MainPhoneButton` _infotainment_menu_72) (`/Game/UMG/Infotainment_Menu.MainMessageButton` _infotainment_menu_72) (`/Game/UMG/Infotainment_Menu.AcceptCallButton` _infotainment_menu_72) (`/Game/UMG/Infotainment_Menu.DeclineCallButton` _infotainment_menu_72) (`/Game/UMG/Infotainment_Menu.VolumeUpButton` _infotainment_menu_72) (`/Game/UMG/Infotainment_Menu.VolumeDownButton` _infotainment_menu_72) (`/Game/UMG/Infotainment_Menu.StationUpButton` _infotainment_menu_72) (`/Game/UMG/Infotainment_Menu.StationDownButton` _infotainment_menu_72) (`/Game/UMG/Infotainment_Menu.Senden1Button` _infotainment_menu_72) (`/Game/UMG/Infotainment_Menu.Senden2Button` _infotainment_menu_72)) (`/Game/UMG/Infotainment_Menu.KeyCounterInfo` _infotainment_menu_72)))
  (bind _item_3 (`KismetArrayLibrary.Array_Get` (`|MakeArray` _urbutton (`/Game/UMG/Navi_Menu.FSButton` _navi_menu_65) (`/Game/UMG/Navi_Menu.TSButton` _navi_menu_65) (`/Game/UMG/Navi_Menu.StartNaviButton` _navi_menu_65) (`/Game/UMG/Navi_Menu.StopNaviButton` _navi_menu_65)) (`/Game/UMG/Navi_Menu.KeyCounterNavi` _navi_menu_65)))
  (bind _item_4 (`KismetArrayLibrary.Array_Get` (`|MakeArray` _klimaminusbutton (`/Game/UMG/Klima_Menu.KlimaPlusButton` _klima_menu) (`/Game/UMG/Klima_Menu.ScheibenHeizungButton` _klima_menu) (`/Game/UMG/Klima_Menu.SitzHeizungButton` _klima_menu)) (`/Game/UMG/Klima_Menu.KeyCounterKlima` _klima_menu)))
  ;[1 1 1] checks gaze
  (if (> _returnvalue_2 380)
    (if (< _returnvalue_2 530)
      (if (> _returnvalue 60)
        (if (< _returnvalue 120)
          (`KismetSystemLibrary.PrintString` "gaze")
          (`Button.SetBackgroundColor` _button_302 (struct :`R` 0.965 :`A` 1.0))
          (`Button.SetColorAndOpacity` _tempomatbuttondown10 (`self.defaultColor`))
          (`Button.SetColorAndOpacity` (`/Game/UMG/Tempomat_menu.TempomatButtonDown1` _tempomat_menu_45) (`self.defaultColor`))
          (`Button.SetColorAndOpacity` (`/Game/UMG/Tempomat_menu.TempomatButtonUp1` _tempomat_menu_45) (`self.defaultColor`))
          (`Button.SetColorAndOpacity` (`/Game/UMG/Tempomat_menu.TempomatButtonUp10` _tempomat_menu_45) (`self.defaultColor`))
          (`Button.SetColorAndOpacity` _item (`self.highlightColor`))
          (`Widget.SetKeyboardFocus` _item)
          (else
            (`Button.SetBackgroundColor` _button_302 (struct :`R` 0.109804 :`G` 0.109804 :`B` 0.109804 :`A` 1.0) :!label _label)))
        (else
          (goto _label)))
      (else
        (goto _label)))
    (else
      (goto _label)))
  (if (> _returnvalue_2 380)
    (if (< _returnvalue_2 530)
      (if (> _returnvalue 170)
        (if (< _returnvalue 220)
          (`KismetSystemLibrary.PrintString` "gaze")
          (`Button.SetBackgroundColor` _button_302_2 (struct :`R` 0.965 :`A` 1.0))
          (`Button.SetColorAndOpacity` _urbutton (`self.defaultColor`))
          (`Button.SetColorAndOpacity` (`/Game/UMG/Navi_Menu.FSButton` _navi_menu_65) (`self.defaultColor`))
          (`Button.SetColorAndOpacity` (`/Game/UMG/Navi_Menu.TSButton` _navi_menu_65) (`self.defaultColor`))
          (`Button.SetColorAndOpacity` (`/Game/UMG/Navi_Menu.StartNaviButton` _navi_menu_65) (`self.defaultColor`))
          (`Button.SetColorAndOpacity` (`/Game/UMG/Navi_Menu.StopNaviButton` _navi_menu_65) (`self.defaultColor`))
          (`Button.SetColorAndOpacity` _item_3 (`self.highlightColor`))
          (`Widget.SetKeyboardFocus` _item_3)
          (`Button.SetColorAndOpacity` _item_3 (struct :`R` 0.965 :`A` 1.0))
          (else
            (`Button.SetBackgroundColor` _button_302_2 (struct :`R` 0.109804 :`G` 0.109804 :`B` 0.109804 :`A` 1.0) :!label _label_2)))
        (else
          (goto _label_2)))
      (else
        (goto _label_2)))
    (else
      (goto _label_2)))
  (if (> _returnvalue_2 720)
    (if (< _returnvalue_2 780)
      (if (> _returnvalue 140)
        (if (< _returnvalue 200)
          (`KismetSystemLibrary.PrintString` "gaze")
          (`Button.SetBackgroundColor` _mainradiobutton (struct :`R` 0.965 :`A` 1.0))
          (`Button.SetBackgroundColor` (`/Game/UMG/Infotainment_Menu.MainPhoneButton` (`/Game/UMG/MainView.Infotainment_Menu_72` (`self.MainViewWidgetReference`))) (struct :`R` 0.965 :`A` 1.0))
          (`Button.SetBackgroundColor` (`/Game/UMG/Infotainment_Menu.MainMessageButton` (`/Game/UMG/MainView.Infotainment_Menu_72` (`self.MainViewWidgetReference`))) (struct :`R` 0.965 :`A` 1.0))
          (`Button.SetColorAndOpacity` _mainradiobutton_2 (`self.defaultColor`))
          (`Button.SetColorAndOpacity` (`/Game/UMG/Infotainment_Menu.MainPhoneButton` _infotainment_menu_72) (`self.defaultColor`))
          (`Button.SetColorAndOpacity` (`/Game/UMG/Infotainment_Menu.MainMessageButton` _infotainment_menu_72) (`self.defaultColor`))
          (`Button.SetColorAndOpacity` (`/Game/UMG/Infotainment_Menu.AcceptCallButton` _infotainment_menu_72) (`self.defaultColor`))
          (`Button.SetColorAndOpacity` (`/Game/UMG/Infotainment_Menu.DeclineCallButton` _infotainment_menu_72) (`self.defaultColor`))
          (`Button.SetColorAndOpacity` (`/Game/UMG/Infotainment_Menu.VolumeUpButton` _infotainment_menu_72) (`self.defaultColor`))
          (`Button.SetColorAndOpacity` (`/Game/UMG/Infotainment_Menu.VolumeDownButton` _infotainment_menu_72) (`self.defaultColor`))
          (`Button.SetColorAndOpacity` (`/Game/UMG/Infotainment_Menu.StationUpButton` _infotainment_menu_72) (`self.defaultColor`))
          (`Button.SetColorAndOpacity` (`/Game/UMG/Infotainment_Menu.StationDownButton` _infotainment_menu_72) (`self.defaultColor`))
          (`Button.SetColorAndOpacity` (`/Game/UMG/Infotainment_Menu.Senden1Button` _infotainment_menu_72) (`self.defaultColor`))
          (`Button.SetColorAndOpacity` (`/Game/UMG/Infotainment_Menu.Senden2Button` _infotainment_menu_72) (`self.defaultColor`))
          (`Button.SetColorAndOpacity` _item_2 (`self.highlightColor`))
          (`Widget.SetKeyboardFocus` _item_2)
          (else
            (`Button.SetBackgroundColor` _mainradiobutton (struct :`R` 0.109804 :`G` 0.109804 :`B` 0.109804 :`A` 1.0) :!label _label_3)
            (`Button.SetBackgroundColor` (`/Game/UMG/Infotainment_Menu.MainPhoneButton` (`/Game/UMG/MainView.Infotainment_Menu_72` (`self.MainViewWidgetReference`))) (struct :`R` 0.109804 :`G` 0.109804 :`B` 0.109804 :`A` 1.0))
            (`Button.SetBackgroundColor` (`/Game/UMG/Infotainment_Menu.MainMessageButton` (`/Game/UMG/MainView.Infotainment_Menu_72` (`self.MainViewWidgetReference`))) (struct :`R` 0.109804 :`G` 0.109804 :`B` 0.109804 :`A` 1.0))))
        (else
          (goto _label_3)))
      (else
        (goto _label_3)))
    (else
      (goto _label_3)))
  (if (> _returnvalue_2 690)
    (if (< _returnvalue_2 800)
      (if (> _returnvalue 250)
        (if (< _returnvalue 370)
          (`KismetSystemLibrary.PrintString` "gaze")
          (`Image.SetColorAndOpacity` _image_72 (struct :`R` 0.965 :`A` 1.0))
          (`Button.SetColorAndOpacity` _klimaminusbutton (`self.defaultColor`))
          (`Button.SetColorAndOpacity` (`/Game/UMG/Klima_Menu.KlimaPlusButton` _klima_menu) (`self.defaultColor`))
          (`Button.SetColorAndOpacity` (`/Game/UMG/Klima_Menu.ScheibenHeizungButton` _klima_menu) (`self.defaultColor`))
          (`Button.SetColorAndOpacity` (`/Game/UMG/Klima_Menu.SitzHeizungButton` _klima_menu) (`self.defaultColor`))
          (`Button.SetColorAndOpacity` _item_4 (`self.highlightColor`))
          (`Widget.SetKeyboardFocus` _item_4)
          (else
            (`Image.SetColorAndOpacity` _image_72 (struct :`R` 0.109804 :`G` 0.109804 :`B` 0.109804 :`A` 1.0) :!label _label_4)))
        (else
          (goto _label_4)))
      (else
        (goto _label_4)))
    (else
      (goto _label_4))))

(event `self.ReceiveBeginPlay`
  (`WidgetBlueprintLibrary.SetInputMode_GameAndUIEx` self)
  (bind _returnvalue (`|CreateWidget` "/Game/UMG/MainView.MainView_C" self self))
  (set `self.MainViewWidgetReference` _returnvalue)
  (`UserWidget.AddToViewport` _returnvalue 0))

(event `/Game/UMG/IHUD.Get Call`
  (`KismetSystemLibrary.Delay` 3.0)
  (`/Game/UMG/Infotainment_Menu.ShowIncomingCall` (`/Game/UMG/MainView.Infotainment_Menu_72` (`self.MainViewWidgetReference`))))

(event `/Game/UMG/IHUD.Get Message`
  (`KismetSystemLibrary.Delay` 3.0)
  (`/Game/UMG/Infotainment_Menu.ShowIncomingMessage` (`/Game/UMG/MainView.Infotainment_Menu_72` (`self.MainViewWidgetReference`))))

(event `/Game/UMG/IHUD.Get Navimeldung`
  (bind _mainviewwidgetreference (`self.MainViewWidgetReference`))
  (`KismetSystemLibrary.Delay` 3.0)
  (`/Game/UMG/Navi_Menu.ShowNavimeldung` (`/Game/UMG/MainView.Navi_Menu_65` _mainviewwidgetreference))
  (`/Game/UMG/Infotainment_Menu.ShowNavimeldung` (`/Game/UMG/MainView.Infotainment_Menu_72` _mainviewwidgetreference)))

(fn `UserConstructionScript`)