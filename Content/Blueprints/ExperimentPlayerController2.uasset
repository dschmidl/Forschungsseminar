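; Player controller for an experiment with an in-car menu UI: cruise control, navigation, infotainment and climate.
; It creates the MainView widget; LB, LT, RB and RT exclusively select a menu through bools.
; Tick highlights and focuses the selected menu's button by its key counter, which D-pad events step, while B focuses back buttons.
; Delayed events trigger call, message and navigation notifications; eye-tracker gaze checks are disconnected despite "gaze" debug prints.
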(event `self.ReceiveTick`
  (params (DeltaSeconds :type "Float (single-precision)"))
  (bind _highlightcolor (`self.highlightColor`))
  (bind _tempomat_menu_45 (`/Game/UMG/MainView.Tempomat_Menu_45` (`self.MainViewWidgetReference`)))
  (bind _navi_menu_65 (`/Game/UMG/MainView.Navi_Menu_65` (`self.MainViewWidgetReference`)))
  (bind _infotainment_menu_72 (`/Game/UMG/MainView.Infotainment_Menu_72` (`self.MainViewWidgetReference`)))
  (bind _infotainment_menu_72_2 (`/Game/UMG/MainView.Infotainment_Menu_72` (`self.MainViewWidgetReference`)))
  (bind _infotainment_menu_72_3 (`/Game/UMG/MainView.Infotainment_Menu_72` (`self.MainViewWidgetReference`)))
  (bind _klima_menu (`/Game/UMG/MainView.Klima_Menu` (`self.MainViewWidgetReference`)))
  (bind _button_302 (`/Game/UMG/Tempomat_menu.Button_302` _tempomat_menu_45))
  (bind _tempomatbuttondown10 (`/Game/UMG/Tempomat_menu.TempomatButtonDown10` _tempomat_menu_45))
  (bind _urbutton (`/Game/UMG/Navi_Menu.URButton` _navi_menu_65))
  (bind _button_302_2 (`/Game/UMG/Navi_Menu.Button_302` _navi_menu_65))
  (bind _klimaminusbutton (`/Game/UMG/Klima_Menu.KlimaMinusButton` _klima_menu))
  (bind _mainradiobutton (`/Game/UMG/Infotainment_Menu.MainRadioButton` _infotainment_menu_72_3))
  (bind _okbutton (`/Game/UMG/Navi_Menu.OkButton` _navi_menu_65))
  (bind _image_72 (`/Game/UMG/Klima_Menu.Image_72` _klima_menu))
  (bind _array (`|MakeArray` (`/Game/UMG/Infotainment_Menu.MainRadioButton` _infotainment_menu_72_2) (`/Game/UMG/Infotainment_Menu.MainPhoneButton` _infotainment_menu_72_2) (`/Game/UMG/Infotainment_Menu.MainMessageButton` _infotainment_menu_72_2) (`/Game/UMG/Infotainment_Menu.AcceptCallButton` _infotainment_menu_72_2) (`/Game/UMG/Infotainment_Menu.DeclineCallButton` _infotainment_menu_72_2) (`/Game/UMG/Infotainment_Menu.VolumeDownButton` _infotainment_menu_72_2) (`/Game/UMG/Infotainment_Menu.VolumeUpButton` _infotainment_menu_72_2) (`/Game/UMG/Infotainment_Menu.StationDownButton` _infotainment_menu_72_2) (`/Game/UMG/Infotainment_Menu.StationUpButton` _infotainment_menu_72_2) (`/Game/UMG/Infotainment_Menu.Senden1Button` _infotainment_menu_72_2) (`/Game/UMG/Infotainment_Menu.Senden2Button` _infotainment_menu_72_2) (`/Game/UMG/Infotainment_Menu.Back4` _infotainment_menu_72_2)))
  (bind _item (`KismetArrayLibrary.Array_Get` (`|MakeArray` _tempomatbuttondown10 (`/Game/UMG/Tempomat_menu.TempomatButtonDown1` _tempomat_menu_45) (`/Game/UMG/Tempomat_menu.TempomatButtonUp1` _tempomat_menu_45) (`/Game/UMG/Tempomat_menu.TempomatButtonUp10` _tempomat_menu_45)) (`KismetMathLibrary.FTrunc` (`/Game/UMG/Tempomat_menu.KeyCounter` _tempomat_menu_45))))
  (bind _item_2 (`KismetArrayLibrary.Array_Get` (`|MakeArray` _urbutton (`/Game/UMG/Navi_Menu.FSButton` _navi_menu_65) (`/Game/UMG/Navi_Menu.TSButton` _navi_menu_65) (`/Game/UMG/Navi_Menu.StartNaviButton` _navi_menu_65) (`/Game/UMG/Navi_Menu.StopNaviButton` _navi_menu_65)) (`/Game/UMG/Navi_Menu.KeyCounterNavi` _navi_menu_65)))
  (bind _item_3 (`KismetArrayLibrary.Array_Get` _array (`/Game/UMG/Infotainment_Menu.KeyCounterInfo` _infotainment_menu_72_2)))
  (bind _item_4 (`KismetArrayLibrary.Array_Get` (`|MakeArray` _klimaminusbutton (`/Game/UMG/Klima_Menu.KlimaPlusButton` _klima_menu) (`/Game/UMG/Klima_Menu.ScheibenHeizungButton` _klima_menu) (`/Game/UMG/Klima_Menu.SitzHeizungButton` _klima_menu)) (`/Game/UMG/Klima_Menu.KeyCounterKlima` _klima_menu)))
  ;[1 1 1] checks gaze
  (if (stale `InputAction|LBButton` _output_get) :!label _label
    (`KismetSystemLibrary.PrintString` "gaze")
    (`Button.SetBackgroundColor` _button_302 (struct :`R` 0.965 :`A` 1.0))
    (`Button.SetBackgroundColor` _tempomatbuttondown10 (`self.defaultColor`))
    (`Button.SetBackgroundColor` (`/Game/UMG/Tempomat_menu.TempomatButtonDown1` _tempomat_menu_45) (`self.defaultColor`))
    (`Button.SetBackgroundColor` (`/Game/UMG/Tempomat_menu.TempomatButtonUp1` _tempomat_menu_45) (`self.defaultColor`))
    (`Button.SetBackgroundColor` (`/Game/UMG/Tempomat_menu.TempomatButtonUp10` _tempomat_menu_45) (`self.defaultColor`))
    (`Button.SetBackgroundColor` _item (`self.highlightColor`))
    (`Widget.SetKeyboardFocus` _item)
    (else
      (`Button.SetBackgroundColor` _button_302 (struct :`R` 0.109804 :`G` 0.109804 :`B` 0.109804 :`A` 1.0))))
  (if (stale `InputAction|LTButton` _output_get) :!label _label_2
    (`KismetSystemLibrary.PrintString` "gaze")
    (`Button.SetBackgroundColor` _button_302_2 (struct :`R` 0.965 :`A` 1.0))
    (`Button.SetBackgroundColor` _urbutton (`self.defaultColor`))
    (`Button.SetBackgroundColor` (`/Game/UMG/Navi_Menu.FSButton` _navi_menu_65) (`self.defaultColor`))
    (`Button.SetBackgroundColor` (`/Game/UMG/Navi_Menu.TSButton` _navi_menu_65) (`self.defaultColor`))
    (`Button.SetBackgroundColor` (`/Game/UMG/Navi_Menu.StartNaviButton` _navi_menu_65) (`self.defaultColor`))
    (`Button.SetBackgroundColor` (`/Game/UMG/Navi_Menu.StopNaviButton` _navi_menu_65) (`self.defaultColor`))
    (`Button.SetBackgroundColor` _item_2 (`self.highlightColor`))
    (if (`Widget.IsVisible` (`/Game/UMG/Navi_Menu.DelayOverlay` _navi_menu_65))
      (`Widget.SetKeyboardFocus` _okbutton)
      (`Button.SetBackgroundColor` _okbutton _highlightcolor)
      (else
        (`Widget.SetKeyboardFocus` _item_2)
        (`Button.SetBackgroundColor` _item_2 _highlightcolor)
        (if (stale `InputAction|RBButton` _output_get) :!label _label_3
          (`KismetSystemLibrary.PrintString` "gaze")
          (`Button.SetBackgroundColor` _mainradiobutton (`self.highlightColor`))
          (`Button.SetBackgroundColor` (`/Game/UMG/Infotainment_Menu.MainPhoneButton` _infotainment_menu_72_3) (`self.highlightColor`))
          (`Button.SetBackgroundColor` (`/Game/UMG/Infotainment_Menu.MainMessageButton` _infotainment_menu_72_3) (`self.highlightColor`))
          (`Image.SetColorAndOpacity` (`/Game/UMG/Infotainment_Menu.Image_1` _infotainment_menu_72_3) (`self.highlightColor`))
          (`Image.SetColorAndOpacity` (`/Game/UMG/Infotainment_Menu.Image_0` _infotainment_menu_72_3) (`self.highlightColor`))
          (`Image.SetColorAndOpacity` (`/Game/UMG/Infotainment_Menu.Image_180` _infotainment_menu_72_3) (`self.highlightColor`))
          (`Image.SetColorAndOpacity` (`/Game/UMG/Infotainment_Menu.Image_264` _infotainment_menu_72_3) (`self.highlightColor`))
          (`Image.SetColorAndOpacity` (`/Game/UMG/Infotainment_Menu.Image_265` _infotainment_menu_72_3) (`self.highlightColor`))
          (`Button.SetBackgroundColor` _array (`self.defaultColor`))
          (`Button.SetBackgroundColor` _item_3 (`self.highlightColor`))
          (`Widget.SetKeyboardFocus` _item_3)
          (`KismetSystemLibrary.PrintString` (`KismetStringLibrary.Conv_IntToString` (`/Game/UMG/Infotainment_Menu.KeyCounterInfo` _infotainment_menu_72)))
          (if (`Widget.IsVisible` (`/Game/UMG/Infotainment_Menu.PhoneCallOverlay` _infotainment_menu_72))
            (`Widget.SetKeyboardFocus` _item_3)
            (`KismetSystemLibrary.PrintString` "" :!label _label_4)
            (if (stale `InputAction|RTButton` _output_get) :!label _label_5
              (`KismetSystemLibrary.PrintString` "gaze")
              (`Image.SetColorAndOpacity` _image_72 (`self.highlightWidgetColor`))
              (`Button.SetBackgroundColor` _klimaminusbutton (`self.defaultColor`))
              (`Button.SetBackgroundColor` (`/Game/UMG/Klima_Menu.KlimaPlusButton` _klima_menu) (`self.defaultColor`))
              (`Button.SetBackgroundColor` (`/Game/UMG/Klima_Menu.ScheibenHeizungButton` _klima_menu) (`self.defaultColor`))
              (`Button.SetBackgroundColor` (`/Game/UMG/Klima_Menu.SitzHeizungButton` _klima_menu) (`self.defaultColor`))
              (`Button.SetBackgroundColor` _item_4 (`self.highlightColor`))
              (`Widget.SetKeyboardFocus` _item_4)
              (else
                (`Image.SetColorAndOpacity` _image_72 (struct :`R` 0.109804 :`G` 0.109804 :`B` 0.109804 :`A` 1.0))))
            (elif (`Widget.IsVisible` (`/Game/UMG/Infotainment_Menu.RadioOverlay` _infotainment_menu_72))
              (`Widget.SetKeyboardFocus` _item_3)
              (goto _label_4)
              (elif (`Widget.IsVisible` (`/Game/UMG/Infotainment_Menu.GetMessageOverlay` _infotainment_menu_72))
                (bind _output_get (set `/Game/UMG/Infotainment_Menu.KeyCounterInfo` 11 _infotainment_menu_72))
                (`Widget.SetKeyboardFocus` (`KismetArrayLibrary.Array_Get` _array _output_get))
                (goto _label_4)
                (elif (`Widget.IsVisible` (`/Game/UMG/Infotainment_Menu.MessageOverlay` _infotainment_menu_72))
                  (if (`Widget.IsVisible` (`/Game/UMG/Infotainment_Menu.Senden1Button` _infotainment_menu_72))
                    (bind _output_get_2 (set `/Game/UMG/Infotainment_Menu.KeyCounterInfo` 9 _infotainment_menu_72))
                    (`Widget.SetKeyboardFocus` (`KismetArrayLibrary.Array_Get` _array _output_get_2))
                    (goto _label_4)
                    (elif (`Widget.IsVisible` (`/Game/UMG/Infotainment_Menu.Senden2Button` _infotainment_menu_72))
                      (bind _output_get_3 (set `/Game/UMG/Infotainment_Menu.KeyCounterInfo` 10 _infotainment_menu_72))
                      (`Widget.SetKeyboardFocus` (`KismetArrayLibrary.Array_Get` _array _output_get_3))
                      (goto _label_4)))))))
          (else
            (`Button.SetBackgroundColor` _mainradiobutton (struct :`R` 0.109804 :`G` 0.109804 :`B` 0.109804 :`A` 1.0))
            (`Button.SetBackgroundColor` (`/Game/UMG/Infotainment_Menu.MainPhoneButton` _infotainment_menu_72_3) (struct :`R` 0.109804 :`G` 0.109804 :`B` 0.109804 :`A` 1.0))
            (`Button.SetBackgroundColor` (`/Game/UMG/Infotainment_Menu.MainMessageButton` _infotainment_menu_72_3) (struct :`R` 0.109804 :`G` 0.109804 :`B` 0.109804 :`A` 1.0))
            (goto _label_5)))))
    (else
      (`Button.SetBackgroundColor` _button_302_2 (struct :`R` 0.109804 :`G` 0.109804 :`B` 0.109804 :`A` 1.0))
      (goto _label_3))))

(event `InputAction|LBButton`
  (params (Key :type "Key Structure" :default "AnyKey"))
  ;[1 1 1] checks gaze
  (:`Pressed`
    (set `self.LTBool` false)
    (set `self.RBBool` false)
    (set `self.RTBool` false))
  (:`Released`
    (bind _output_get (set `self.LBBool` true))
    (goto _label)))

(event `InputAction|dpadDown`
  (params (Key :type "Key Structure" :default "AnyKey"))
  (bind _tempomat_menu_45 (`/Game/UMG/MainView.Tempomat_Menu_45` (`self.MainViewWidgetReference`)))
  (:`Released`
    (if (`Widget.HasKeyboardFocus` (`KismetArrayLibrary.Array_Get` (`|MakeArray` (`/Game/UMG/Tempomat_menu.TempomatButtonDown10` _tempomat_menu_45) (`/Game/UMG/Tempomat_menu.TempomatButtonDown1` _tempomat_menu_45) (`/Game/UMG/Tempomat_menu.TempomatButtonUp1` _tempomat_menu_45) (`/Game/UMG/Tempomat_menu.TempomatButtonUp10` _tempomat_menu_45)) (`KismetMathLibrary.FTrunc` (`/Game/UMG/Tempomat_menu.KeyCounter` _tempomat_menu_45))))
      (`/Game/UMG/Tempomat_menu.SetCounterTempoUp` (`/Game/UMG/MainView.Tempomat_Menu_45` (`self.MainViewWidgetReference`))))))

(event `InputAction|dpadUp`
  (params (Key :type "Key Structure" :default "AnyKey"))
  (bind _tempomat_menu_45 (`/Game/UMG/MainView.Tempomat_Menu_45` (`self.MainViewWidgetReference`)))
  (:`Released`
    (if (`Widget.HasKeyboardFocus` (`KismetArrayLibrary.Array_Get` (`|MakeArray` (`/Game/UMG/Tempomat_menu.TempomatButtonDown10` _tempomat_menu_45) (`/Game/UMG/Tempomat_menu.TempomatButtonDown1` _tempomat_menu_45) (`/Game/UMG/Tempomat_menu.TempomatButtonUp1` _tempomat_menu_45) (`/Game/UMG/Tempomat_menu.TempomatButtonUp10` _tempomat_menu_45)) (`KismetMathLibrary.FTrunc` (`/Game/UMG/Tempomat_menu.KeyCounter` _tempomat_menu_45))))
      (`/Game/UMG/Tempomat_menu.SetCounterTempoDown` (`/Game/UMG/MainView.Tempomat_Menu_45` (`self.MainViewWidgetReference`))))))

(event `InputAction|LTButton`
  (params (Key :type "Key Structure" :default "AnyKey"))
  (:`Pressed`
    ;[1 1 1] checks gaze
    (set `self.LBBool` false)
    (set `self.RBBool` false)
    (set `self.RTBool` false))
  (:`Released`
    (bind _output_get (set `self.LTBool` true))
    (goto _label_2)))

(event `InputAction|dpadDown`
  (params (Key :type "Key Structure" :default "AnyKey"))
  (bind _navi_menu_65 (`/Game/UMG/MainView.Navi_Menu_65` (`self.MainViewWidgetReference`)))
  (:`Released`
    (if (`Widget.HasKeyboardFocus` (`KismetArrayLibrary.Array_Get` (`|MakeArray` (`/Game/UMG/Navi_Menu.URButton` _navi_menu_65) (`/Game/UMG/Navi_Menu.FSButton` _navi_menu_65) (`/Game/UMG/Navi_Menu.TSButton` _navi_menu_65) (`/Game/UMG/Navi_Menu.StartNaviButton` _navi_menu_65) (`/Game/UMG/Navi_Menu.StopNaviButton` _navi_menu_65)) (`/Game/UMG/Navi_Menu.KeyCounterNavi` _navi_menu_65)))
      (`/Game/UMG/Navi_Menu.SetCounterNaviUp` (`/Game/UMG/MainView.Navi_Menu_65` (`self.MainViewWidgetReference`))))))

(event `InputAction|dpadUp`
  (params (Key :type "Key Structure" :default "AnyKey"))
  (bind _navi_menu_65 (`/Game/UMG/MainView.Navi_Menu_65` (`self.MainViewWidgetReference`)))
  (:`Released`
    (if (`Widget.HasKeyboardFocus` (`KismetArrayLibrary.Array_Get` (`|MakeArray` (`/Game/UMG/Navi_Menu.URButton` _navi_menu_65) (`/Game/UMG/Navi_Menu.FSButton` _navi_menu_65) (`/Game/UMG/Navi_Menu.TSButton` _navi_menu_65) (`/Game/UMG/Navi_Menu.StartNaviButton` _navi_menu_65) (`/Game/UMG/Navi_Menu.StopNaviButton` _navi_menu_65)) (`/Game/UMG/Navi_Menu.KeyCounterNavi` _navi_menu_65)))
      (`/Game/UMG/Navi_Menu.SetCounterNaviDown` (`/Game/UMG/MainView.Navi_Menu_65` (`self.MainViewWidgetReference`))))))

(event `InputAction|RBButton`
  (params (Key :type "Key Structure" :default "AnyKey"))
  (:`Pressed`
    (set `self.LBBool` false)
    (set `self.LTBool` false)
    (set `self.RTBool` false))
  (:`Released`
    (bind _output_get (set `self.RBBool` true))
    (goto _label_3)))

(event `InputAction|RTButton`
  (params (Key :type "Key Structure" :default "AnyKey"))
  (:`Pressed`
    (set `self.LBBool` false)
    (set `self.LTBool` false)
    (set `self.RBBool` false))
  (:`Released`
    (bind _output_get (set `self.RTBool` true))
    (goto _label_5)))

(event `InputAction|BButtonPressed`
  (params (Key :type "Key Structure" :default "AnyKey"))
  (:`Released`
    (`Widget.SetKeyboardFocus` (`/Game/UMG/Infotainment_Menu.Back1` (`/Game/UMG/MainView.Infotainment_Menu_72` (`self.MainViewWidgetReference`))))
    (`Widget.SetKeyboardFocus` (`/Game/UMG/Infotainment_Menu.BackButton2` (`/Game/UMG/MainView.Infotainment_Menu_72` (`self.MainViewWidgetReference`))))
    (`Widget.SetKeyboardFocus` (`/Game/UMG/Infotainment_Menu.Back3` (`/Game/UMG/MainView.Infotainment_Menu_72` (`self.MainViewWidgetReference`))))
    (`Widget.SetKeyboardFocus` (`/Game/UMG/Infotainment_Menu.Back4` (`/Game/UMG/MainView.Infotainment_Menu_72` (`self.MainViewWidgetReference`))))))

(event `InputAction|dpadDown`
  (params (Key :type "Key Structure" :default "AnyKey"))
  (bind _infotainment_menu_72 (`/Game/UMG/MainView.Infotainment_Menu_72` (`self.MainViewWidgetReference`)))
  (bind _infotainment_menu_72_2 (`/Game/UMG/MainView.Infotainment_Menu_72` (`self.MainViewWidgetReference`)))
  (:`Released`
    (if (`Widget.HasKeyboardFocus` (`KismetArrayLibrary.Array_Get` (`|MakeArray` (`/Game/UMG/Infotainment_Menu.MainRadioButton` _infotainment_menu_72_2) (`/Game/UMG/Infotainment_Menu.MainPhoneButton` _infotainment_menu_72_2) (`/Game/UMG/Infotainment_Menu.MainMessageButton` _infotainment_menu_72_2) (`/Game/UMG/Infotainment_Menu.AcceptCallButton` _infotainment_menu_72_2) (`/Game/UMG/Infotainment_Menu.DeclineCallButton` _infotainment_menu_72_2) (`/Game/UMG/Infotainment_Menu.VolumeDownButton` _infotainment_menu_72_2) (`/Game/UMG/Infotainment_Menu.VolumeUpButton` _infotainment_menu_72_2) (`/Game/UMG/Infotainment_Menu.StationDownButton` _infotainment_menu_72_2) (`/Game/UMG/Infotainment_Menu.StationUpButton` _infotainment_menu_72_2) (`/Game/UMG/Infotainment_Menu.Senden1Button` _infotainment_menu_72_2) (`/Game/UMG/Infotainment_Menu.Senden2Button` _infotainment_menu_72_2) (`/Game/UMG/Infotainment_Menu.Back4` _infotainment_menu_72_2)) (`/Game/UMG/Infotainment_Menu.KeyCounterInfo` _infotainment_menu_72_2)))
      (`/Game/UMG/Infotainment_Menu.SetCounterInfoUp` _infotainment_menu_72)
      (`/Game/UMG/Infotainment_Menu.PhoneCallUp` _infotainment_menu_72))))

(event `InputAction|dpadUp`
  (params (Key :type "Key Structure" :default "AnyKey"))
  (bind _infotainment_menu_72 (`/Game/UMG/MainView.Infotainment_Menu_72` (`self.MainViewWidgetReference`)))
  (bind _infotainment_menu_72_2 (`/Game/UMG/MainView.Infotainment_Menu_72` (`self.MainViewWidgetReference`)))
  (:`Released`
    (if (`Widget.HasKeyboardFocus` (`KismetArrayLibrary.Array_Get` (`|MakeArray` (`/Game/UMG/Infotainment_Menu.MainRadioButton` _infotainment_menu_72_2) (`/Game/UMG/Infotainment_Menu.MainPhoneButton` _infotainment_menu_72_2) (`/Game/UMG/Infotainment_Menu.MainMessageButton` _infotainment_menu_72_2) (`/Game/UMG/Infotainment_Menu.AcceptCallButton` _infotainment_menu_72_2) (`/Game/UMG/Infotainment_Menu.DeclineCallButton` _infotainment_menu_72_2) (`/Game/UMG/Infotainment_Menu.VolumeDownButton` _infotainment_menu_72_2) (`/Game/UMG/Infotainment_Menu.VolumeUpButton` _infotainment_menu_72_2) (`/Game/UMG/Infotainment_Menu.StationDownButton` _infotainment_menu_72_2) (`/Game/UMG/Infotainment_Menu.StationUpButton` _infotainment_menu_72_2) (`/Game/UMG/Infotainment_Menu.Senden1Button` _infotainment_menu_72_2) (`/Game/UMG/Infotainment_Menu.Senden2Button` _infotainment_menu_72_2) (`/Game/UMG/Infotainment_Menu.Back4` _infotainment_menu_72_2)) (`/Game/UMG/Infotainment_Menu.KeyCounterInfo` _infotainment_menu_72_2)))
      (`/Game/UMG/Infotainment_Menu.SetCounterInfoDown` _infotainment_menu_72)
      (`/Game/UMG/Infotainment_Menu.PhoneCallDown` _infotainment_menu_72))))

(event `InputAction|dpadDown`
  (params (Key :type "Key Structure" :default "AnyKey"))
  (bind _klima_menu (`/Game/UMG/MainView.Klima_Menu` (`self.MainViewWidgetReference`)))
  (:`Released`
    (if (`Widget.HasKeyboardFocus` (`KismetArrayLibrary.Array_Get` (`|MakeArray` (`/Game/UMG/Klima_Menu.KlimaMinusButton` _klima_menu) (`/Game/UMG/Klima_Menu.KlimaPlusButton` _klima_menu) (`/Game/UMG/Klima_Menu.ScheibenHeizungButton` _klima_menu) (`/Game/UMG/Klima_Menu.SitzHeizungButton` _klima_menu)) (`/Game/UMG/Klima_Menu.KeyCounterKlima` _klima_menu)))
      (`/Game/UMG/Klima_Menu.SetCounterKlimaUp` (`/Game/UMG/MainView.Klima_Menu` (`self.MainViewWidgetReference`))))))

(event `InputAction|dpadUp`
  (params (Key :type "Key Structure" :default "AnyKey"))
  (bind _klima_menu (`/Game/UMG/MainView.Klima_Menu` (`self.MainViewWidgetReference`)))
  (:`Released`
    (if (`Widget.HasKeyboardFocus` (`KismetArrayLibrary.Array_Get` (`|MakeArray` (`/Game/UMG/Klima_Menu.KlimaMinusButton` _klima_menu) (`/Game/UMG/Klima_Menu.KlimaPlusButton` _klima_menu) (`/Game/UMG/Klima_Menu.ScheibenHeizungButton` _klima_menu) (`/Game/UMG/Klima_Menu.SitzHeizungButton` _klima_menu)) (`/Game/UMG/Klima_Menu.KeyCounterKlima` _klima_menu)))
      (`/Game/UMG/Klima_Menu.SetCounterKlimaDown` (`/Game/UMG/MainView.Klima_Menu` (`self.MainViewWidgetReference`))))))

(event `self.ReceiveBeginPlay`
  (`WidgetBlueprintLibrary.SetInputMode_GameAndUIEx` self)
  (bind _returnvalue (`|CreateWidget` "/Game/UMG/MainView.MainView_C" self self))
  (set `self.MainViewWidgetReference` _returnvalue)
  (`UserWidget.AddToViewport` _returnvalue 0))

(event `/Game/UMG/IHUD.Get Call`
  (`KismetSystemLibrary.Delay` 3.0)
  (`/Game/UMG/Infotainment_Menu.ShowIncomingCall` (`/Game/UMG/MainView.Infotainment_Menu_72` (`self.MainViewWidgetReference`))))

(event `/Game/UMG/IHUD.Get Message`
  (`KismetSystemLibrary.Delay` 3.0)
  (`/Game/UMG/Infotainment_Menu.ShowIncomingMessage` (`/Game/UMG/MainView.Infotainment_Menu_72` (`self.MainViewWidgetReference`))))

(event `/Game/UMG/IHUD.Get Navimeldung`
  (bind _mainviewwidgetreference (`self.MainViewWidgetReference`))
  (`KismetSystemLibrary.Delay` 3.0)
  (`/Game/UMG/Navi_Menu.ShowNavimeldung` (`/Game/UMG/MainView.Navi_Menu_65` _mainviewwidgetreference))
  (`/Game/UMG/Infotainment_Menu.ShowNavimeldung` (`/Game/UMG/MainView.Infotainment_Menu_72` _mainviewwidgetreference)))

(fn `UserConstructionScript`)