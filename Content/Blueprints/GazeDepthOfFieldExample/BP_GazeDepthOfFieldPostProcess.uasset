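; Post process actor that drives gaze-contingent depth of field from EyeX eye tracking.
; Each tick it reads the EyeX player controller's gaze hit and projects the camera-to-hit vector onto the camera forward to get focal distance.
; Current focus eases toward that distance with FInterpTo, holding when there is no valid hit.
; It then rewrites the global post process settings, using the focal distance for both transition regions too.
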(event `self.ReceiveTick`
  (params (DeltaSeconds :type "Float (single-precision)"))
  (bind _returnvalue (`GameplayStatics.GetPlayerCameraManager` 0))
  (bind _gazefocaldistance (`self.GazeFocalDistance`))
  (bind _currentfocaldistance (`self.CurrentFocalDistance`))
  (`|ExecutionSequence`
    (:`then_0`
      ;[1 1 1] Calculate new focal distance
      (bind _asbp_eye_xplayer_controller_do_f (cast `/Game/Blueprints/GazeDepthOfFieldExample/BP_EyeXPlayerControllerDoF` (`GameplayStatics.GetPlayerController` 0)))
      (bind (_impactpoint _hitactor _bisvalid) (`EyeXPlayerController.GetGazeHitResult` _asbp_eye_xplayer_controller_do_f))
      (if _bisvalid
        (set `self.GazeFocalDistance` (`KismetMathLibrary.VSize` (`KismetMathLibrary.ProjectVectorOnToVector` (- (`self.K2_GetActorLocation` _returnvalue) _impactpoint) (`self.GetActorForwardVector` _returnvalue))))
        (else
          (set `self.GazeFocalDistance` 0.0))))
    (:`then_1`
      ;[1 1 1] Interpolate towards new focal distance
      (if (!= _gazefocaldistance 0.0)
        (set `self.CurrentFocalDistance` (`KismetMathLibrary.FInterpTo` (`self.CurrentFocalDistance`) _gazefocaldistance (`GameplayStatics.GetWorldDeltaSeconds`) (`self.InterpSpeed`)))))
    (:`then_2`
      ;[1 1 1] Update Post Process
      (set `PostProcessComponent.Settings` (make `PostProcessSettings` :`bOverride_DepthOfFieldFocalDistance` true :`DepthOfFieldFocalDistance` _currentfocaldistance :`bOverride_DepthOfFieldNearTransitionRegion` true :`DepthOfFieldNearTransitionRegion` _currentfocaldistance :`bOverride_DepthOfFieldFarTransitionRegion` true :`DepthOfFieldFarTransitionRegion` _currentfocaldistance :`bOverride_DepthOfFieldScale` true :`DepthOfFieldScale` (`self.Scale`) :`bOverride_DepthOfFieldMaxBokehSize` true :`DepthOfFieldMaxBokehSize` (`self.MaxBokehSize`)) (`self.GazeDepthOfFieldPostProcessGlobal`)))))

(fn `UserConstructionScript`)