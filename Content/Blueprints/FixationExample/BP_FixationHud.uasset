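; Example HUD that visualizes EyeX eye-tracker fixations on screen beneath a title and help text.
; Each draw, it stores a newly completed fixation, detected by timestamp, in a ring buffer of recent fixations.
; An extra last slot holds the ongoing fixation, toggled with the O key.
; Valid entries are drawn as textures centered on their gaze points, sized by clamped duration, with a distinct texture for the ongoing one.
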(event `self.ReceiveBeginPlay`
  ;[1 1 1] Enable input for this blueprint
  (`self.EnableInput` (`GameplayStatics.GetPlayerController` 0)))

(event `Key|O`
  (params (Key :type "Key Structure"))
  ;[1 1 1] Toggle ShowOngoingFixation when 'o' pressed.
  (:`Pressed`
    (set `self.ShowOngoingFixation` (not (`self.ShowOngoingFixation`)))))

(event `self.ReceiveDrawHUD`
  (params (SizeX :type Integer) (SizeY :type Integer))
  (bind (_gazepoint _begintimestamp _duration _bhasvalue) (`EyeXBlueprintLibrary.GetLastFixation` "Sensitive"))
  (bind (_gazepoint_2 _begintimestamp_2 _duration_2 _bhasvalue_2) (`EyeXBlueprintLibrary.GetOngoingFixation` "Sensitive"))
  (bind _fixationtexturesize (`self.FixationTextureSize`))
  ;[1 1 1] Print help text.
  (bind (_screen_x _screen_y _outwidth _outheight) (`/Game/Blueprints/BPMacroLibrary.DrawCenteredTextOnHUD` (/ SizeX 2) (/ SizeY 3) "Fixations" (struct :`R` 1.0 :`G` 1.0 :`B` 1.0 :`A` 1.0) "/Game/Fonts/Calibri.Calibri")
    (:`  `
      (`self.DrawText` (`self.HelpText`) (struct :`R` 1.0 :`G` 1.0 :`B` 1.0 :`A` 1.0) _screen_x (+ _screen_y _outheight) "/Game/Fonts/Calibri_small.Calibri_small")
      (`|ExecutionSequence`
        (:`then_0`
          ;[1 1 1] Retrieve last fixation and check if valid and different from last saved fixation
          (set `self.LastFixationBeginTimestamp` _begintimestamp)
          (if _bhasvalue
            (set `self.LastFixation` (make `EyeXFixationDataPoint` _gazepoint _begintimestamp _duration _bhasvalue))
            ;;[1 1 1] Different from last saved fixation?
            (`/Engine/EditorBlueprintResources/StandardMacros.CompareFloat` (`self.LastFixationBeginTimestamp`) (`self.LastSavedTimeStamp`)
              (:`>`
                ;[1 1 1] If different last fixation: Save new timestamp and save last fixation to array.
                (set `self.LastSavedTimeStamp` (`self.LastFixationBeginTimestamp`))
                (set `self.TotalNumberOfFixations` (+ (`self.TotalNumberOfFixations`) 1))
                (`KismetArrayLibrary.Array_Set` (`self.SavedFixations`) (mod (`self.TotalNumberOfFixations`) (`self.NumberOfFixationsToSave`)) (`self.LastFixation`))))))
        (:`then_1`
          ;[1 1 1] If ShowOngoingFixation is true: set ongoing fixation as last entry in array; else set last entry to invalid fixation.
          (if (`self.ShowOngoingFixation`)
            (`KismetArrayLibrary.Array_Set` (`self.SavedFixations`) (`self.NumberOfFixationsToSave`) (make `EyeXFixationDataPoint` _gazepoint_2 _begintimestamp_2 _duration_2 _bhasvalue_2) true)
            (else
              (`KismetArrayLibrary.Array_Set` (`self.SavedFixations`) (`self.NumberOfFixationsToSave`) (`self.InvalidFixation`) true))))
        (:`then_2`
          ;[1 1 1] Draw last five valid fixations on screen, with size according to fixation duration. And draw current fixation on top of the five fixations. Current fixation will be moving around a bit.
          (for (_array_element _array_index) (`self.SavedFixations`)
            (bind (_gazepoint_3 _begintimestamp_3 _duration_3 _bhasvalue_3) (break `EyeXFixationDataPoint` _array_element))
            ;;[1 1 1] Is valid fixation?
            (if _bhasvalue_3
              ;;[1 1 1] Is current array index for ongoing fixation?
              (if (== _array_index (`self.NumberOfFixationsToSave`))
                (bind (_x _y) (`KismetMathLibrary.BreakVector2D` _gazepoint_3))
                (bind _returnvalue (`KismetMathLibrary.MapRangeUnclamped` (`KismetMathLibrary.FClamp` _duration_3 0.0 1500.0) 0.0 1500.0 _fixationtexturesize (* 3 _fixationtexturesize)))
                (bind _returnvalue_2 (/ _returnvalue 2.0))
                (bind _returnvalue_3 (- _x _returnvalue_2))
                (bind _returnvalue_4 (- _y _returnvalue_2))
                (`self.DrawTexture` "/Game/Textures/FixationPoint_current.FixationPoint_current" _returnvalue_3 _returnvalue_4 _returnvalue _returnvalue 0.0 0.0 1.0 1.0 (struct :`R` 0.995 :`G` 0.995 :`B` 0.995 :`A` 1.0))
                (else
                  (`self.DrawTexture` "/Game/Textures/FixationPoint_saved.FixationPoint_saved" _returnvalue_3 _returnvalue_4 _returnvalue _returnvalue 0.0 0.0 1.0 1.0 (struct :`R` 0.995 :`G` 0.995 :`B` 0.995 :`A` 1.0)))))))))))

(fn `UserConstructionScript`)